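; Base weapon Blueprint for an FPS, handling firing, ammo, reloading and aim state from player character events, and driving the player's ADS FOV each tick.
; WeaponFire spends ammo, then fires single or multiple hitscan shots with impact effects and damage messages, or spawns a projectile.
; CalculateShot traces from the camera with random spread, orienting projectiles from muzzle toward the hit.
; Automatic weapons add timeline-driven pitch recoil that reverses to recover.
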(event Custom|AutomaticRecoil
  (bind _returnvalue (Game|Player|GetPlayerPawn 0))
  (bind (_direction _alpha) (Timeline|RecoilTimeline PlayFromStart)
    (:Update
      (switch Utilities|FlowControl|Switch|SwitchonETimelineDirection _direction
        (:Forward
          (Pawn|Input|AddControllerPitchInput _returnvalue (Math|Float|Lerp 0.0 (Variables|Recoil|GetRecoilPitch) _alpha)))
        (:Backward
          (Pawn|Input|AddControllerPitchInput _returnvalue (* (Math|Float|Lerp 0.0 (Variables|Recoil|GetRecoilPitch) _alpha) -1.0)))))
    (:Finished
      (CallFunction|ReverseRecoil)
      (Utilities|FlowControl|RetriggerableDelay 0.05)
      (CallFunction|StopRecoil))))

(event Custom|StopRecoil
  (bind _returnvalue (Game|Player|GetPlayerPawn 0))
  (bind (_direction _alpha) (Timeline|RecoilTimeline Stop)
    (:Update
      (switch Utilities|FlowControl|Switch|SwitchonETimelineDirection _direction
        (:Forward
          (Pawn|Input|AddControllerPitchInput _returnvalue (Math|Float|Lerp 0.0 (Variables|Recoil|GetRecoilPitch) _alpha)))
        (:Backward
          (Pawn|Input|AddControllerPitchInput _returnvalue (* (Math|Float|Lerp 0.0 (Variables|Recoil|GetRecoilPitch) _alpha) -1.0)))))
    (:Finished
      (CallFunction|ReverseRecoil)
      (Utilities|FlowControl|RetriggerableDelay 0.05)
      (CallFunction|StopRecoil))))

(event Custom|ReverseRecoil
  (bind _returnvalue (Game|Player|GetPlayerPawn 0))
  (bind (_direction _alpha) (Timeline|RecoilTimeline Reverse)
    (:Update
      (switch Utilities|FlowControl|Switch|SwitchonETimelineDirection _direction
        (:Forward
          (Pawn|Input|AddControllerPitchInput _returnvalue (Math|Float|Lerp 0.0 (Variables|Recoil|GetRecoilPitch) _alpha)))
        (:Backward
          (Pawn|Input|AddControllerPitchInput _returnvalue (* (Math|Float|Lerp 0.0 (Variables|Recoil|GetRecoilPitch) _alpha) -1.0)))))
    (:Finished
      (CallFunction|ReverseRecoil)
      (Utilities|FlowControl|RetriggerableDelay 0.05)
      (CallFunction|StopRecoil))))

(event Custom|OnAimEnter
  (Variables|ADS|SetisAiming true))

(event Custom|OnAimExit
  (Variables|ADS|SetisAiming false))

(event EventBeginPlay
  (bind _asfps_character (Utilities|Casting|CastToFPS_Character (Game|Player|GetPlayerPawn 0)))
  (Variables|References|SetPlayerRef _asfps_character)
  (EventDispatchers|BindEventtoAimEnter _asfps_character (delegate Custom|OnAimEnter))
  (EventDispatchers|BindEventtoAimExit _asfps_character (delegate Custom|OnAimExit)))

(event EventTick
  (params (DeltaSeconds :type Float%20%28single-precision%29))
  (Default|ADSFOV (Variables|References|GetPlayerRef)))

(fn ConstructionScript)

(fn WeaponFire
  (params (FireType :type FireType%20Enum :default "NewEnumerator0"))
  (Variables|Ammo|SetCurrentAmmo (- (Variables|Ammo|GetCurrentAmmo) 1))
  (switch Utilities|FlowControl|Switch|SwitchonFireType FireType
    (:NewEnumerator0
      (if (Variables|Ammo|GetMultipleBullets)
        (for _index (range 0 (- (Variables|Ammo|GetBulletCount) 1))
          (bind _hitresult (CallFunction|CalculateShot (Variables|/Game/Blueprints/FPS_Character.FPS_Character_C|GetCamera (Variables|References|GetPlayerRef)) (Variables|Default|GetGunMesh) "MuzzleFlash"))
          (Game|SpawnActorfromClass (Variables|References|GetImpactEffectClass) (Math|Transform|MakeTransform (.ImpactPoint (Collision|BreakHitResult _hitresult)) "0, 0, 0" "1,1,1") "Undefined" 0 _hitresult (.bBlockingHit (Collision|BreakHitResult _hitresult)) 0)
          (CallFunction|AddDamage _hitresult)
          (if (Variables|Properties|GetisAutomaticWeapon)
            (CallFunction|AutomaticRecoil)))
        (else
          (bind _hitresult_2 (CallFunction|CalculateShot (Variables|/Game/Blueprints/FPS_Character.FPS_Character_C|GetCamera (Variables|References|GetPlayerRef)) (Variables|Default|GetGunMesh) "MuzzleFlash"))
          (Game|SpawnActorfromClass (Variables|References|GetImpactEffectClass) (Math|Transform|MakeTransform (.ImpactPoint (Collision|BreakHitResult _hitresult_2)) "0, 0, 0" "1,1,1") "Undefined" 0 _hitresult_2 (.bBlockingHit (Collision|BreakHitResult _hitresult_2)) 0)
          (CallFunction|AddDamage _hitresult_2)
          (if (Variables|Properties|GetisAutomaticWeapon) :!label _label
            (CallFunction|AutomaticRecoil)))))
    (:NewEnumerator1
      (bind _projectiletransform (CallFunction|CalculateShot (Variables|/Game/Blueprints/FPS_Character.FPS_Character_C|GetCamera (Variables|References|GetPlayerRef)) (Variables|Default|GetGunMesh) "MuzzleFlash"))
      (bind _returnvalue (Game|SpawnActorfromClass (Variables|Projectile|GetProjectile) _projectiletransform "Undefined" 0 (Variables|Properties|GetAmmoData) (Variables|Stats|GetCriticalHitDamageModifier) 0))
      (Variables|Projectile|SetSpawnProjectile _returnvalue)
      (goto _label))))

(fn WeaponReload
  (Variables|Ammo|SetCurrentAmmo (Math|Integer|Min(Integer) (Variables|Ammo|GetMaxMagAmmo) (Variables|Ammo|GetCurrentTotalAmmo)))
  (Variables|Ammo|SetCurrentTotalAmmo (- (Variables|Ammo|GetCurrentTotalAmmo) (Math|Integer|Min(Integer) (Variables|Ammo|GetMaxMagAmmo) (Variables|Ammo|GetCurrentTotalAmmo)))))

(fn HasAmmoinMag
  (return (> (Variables|Ammo|GetCurrentAmmo) 0) (== (Variables|Ammo|GetCurrentAmmo) (Variables|Ammo|GetMaxMagAmmo))))

(fn HasExtraAmmo
  (return (> (Variables|Ammo|GetCurrentTotalAmmo) 0)))

(fn CalculateShot
  (params (Camera :type Camera%20Component%20Object%20Reference) (WeaponMesh :type Scene%20Component%20Object%20Reference) (WeaponFireSocketName :type Name))
  (bind _bulletspread (Variables|Stats|GetBulletSpread))
  (bind _returnvalue (* _bulletspread -1.0))
  (Utilities|FlowControl|Sequence
    (:then_0
      (LocalVariables|SetLocalCamera Camera)
      (LocalVariables|SetLocalWeaponMesh WeaponMesh)
      (LocalVariables|SetLocalSocketNAme WeaponFireSocketName))
    (:then_1
      (bind (_outhit _returnvalue_2) (Collision|LineTraceForObjects (.location (Transformation|GetWorldTransform (LocalVariables|GetLocalCamera))) (Math|Vector|MakeVector (+ (.X (Math|Vector|BreakVector (+ (.location (Transformation|GetWorldTransform (LocalVariables|GetLocalCamera))) (* (Math|Vector|GetForwardVector (.rotation (Transformation|GetWorldTransform (LocalVariables|GetLocalCamera)))) 1e+04)))) (Math|Random|RandomFloatinRange _returnvalue _bulletspread)) (+ (.Y (Math|Vector|BreakVector (+ (.location (Transformation|GetWorldTransform (LocalVariables|GetLocalCamera))) (* (Math|Vector|GetForwardVector (.rotation (Transformation|GetWorldTransform (LocalVariables|GetLocalCamera)))) 1e+04)))) (Math|Random|RandomFloatinRange _returnvalue _bulletspread)) (+ (.Z (Math|Vector|BreakVector (+ (.location (Transformation|GetWorldTransform (LocalVariables|GetLocalCamera))) (* (Math|Vector|GetForwardVector (.rotation (Transformation|GetWorldTransform (LocalVariables|GetLocalCamera)))) 1e+04)))) (Math|Random|RandomFloatinRange _returnvalue _bulletspread))) (Utilities|Array|MakeArray "ObjectTypeQuery1" "ObjectTypeQuery2") false (Utilities|Array|MakeArray (Game|Player|GetPlayerPawn 0)) "None"))
      (if _returnvalue_2
        (LocalVariables|SetLocalProjectileTransform (Math|Transform|MakeTransform (Transformation|GetSocketLocation (LocalVariables|GetLocalWeaponMesh) (LocalVariables|GetLocalSocketNAme)) (Math|Rotator|FindLookatRotation (Transformation|GetSocketLocation (LocalVariables|GetLocalWeaponMesh) (LocalVariables|GetLocalSocketNAme)) (.ImpactPoint (Collision|BreakHitResult _outhit)))))
        (else
          (LocalVariables|SetLocalProjectileTransform (Math|Transform|MakeTransform (Transformation|GetSocketLocation (LocalVariables|GetLocalWeaponMesh) (LocalVariables|GetLocalSocketNAme)) (Pawn|GetControlRotation (.AsPawn (Utilities|Casting|CastToPawn (Components|GetOwner (LocalVariables|GetLocalCamera)))) :!class /Script/Engine.Pawn))))))
    (:then_2
      (return _outhit (LocalVariables|GetLocalProjectileTransform)))))

(fn AddDamage
  (params (HitResult :type Hit%20Result%20Structure))
  (Class|TakeDamage|TakeDamage(Message) (.HitActor (Collision|BreakHitResult HitResult)) (Variables|Properties|GetAmmoData) (Variables|Stats|GetCriticalHitDamageModifier) HitResult))

(fn StopFire)