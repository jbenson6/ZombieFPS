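; Grenade launcher weapon Blueprint that extends parent weapon behavior with launcher-specific ammo, animation, sound and recoil.
; On BeginPlay it pulls its ammo data from FPS_GameInstance.
; Firing plays the gun mesh's fire animation and reloading plays a reload sound at the world origin, both after the parent logic.
; Aiming halves recoil intensity and leaving aim restores it, each set before calling the parent handler.
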(event EventBeginPlay
  (|CallParentFunction)
  (bind _asfps_game_instance (Utilities|Casting|CastToFPS_GameInstance (Game|GetGameInstance)))
  (Variables|Default|SetAmmoData (Variables|/Game/Blueprints/FPS_GameInstance.FPS_GameInstance_C|GetGrendadeLauncherAmmoData _asfps_game_instance)))

(event EventWeaponFire
  (params (FireType :type FireType%20Enum :default "NewEnumerator0"))
  (|CallParentFunction FireType)
  (Components|Animation|PlayAnimation (Variables|Default|GetGunMesh) "/Game/MilitaryWeapSilver/Weapons/Animations/Fire_GrenadeLauncher_W.Fire_GrenadeLauncher_W" false))

(event EventWeaponReload
  (|CallParentFunction)
  (Audio|PlaySoundatLocation "/Game/MilitaryWeapSilver/Sound/GrenadeLauncher/Wavs/GrenadeLauncher_Reload03.GrenadeLauncher_Reload03" "0, 0, 0" "0, 0, 0" 1.0 1.0 0.0 0 0 0))

(event EventOnAimEnter
  (Variables|Default|SetRecoilIntesity 3e+01)
  (|CallParentFunction))

(event EventOnAimExit
  (Variables|Default|SetRecoilIntesity 6e+01)
  (|CallParentFunction))

(fn ConstructionScript
  (|CallParentFunction))