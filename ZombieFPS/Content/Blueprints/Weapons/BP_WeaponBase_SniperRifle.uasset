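; Sniper rifle weapon Blueprint, a child weapon that loads its ammo data from the game instance on BeginPlay.
; Firing plays the gun animation, then applies automatic recoil when aimed or ejects a shell effect from the hip.
; Aiming swaps the HUD, player and gun mesh for a scope widget after a short delay, removes bullet spread, lowers recoil and locks weapon switching and reloading until aim exit.
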(event EventBeginPlay
  (|CallParentFunction)
  (bind _asfps_game_instance (Utilities|Casting|CastToFPS_GameInstance (Game|GetGameInstance)))
  (Variables|Default|SetAmmoData (Variables|/Game/Blueprints/FPS_GameInstance.FPS_GameInstance_C|GetSniperRifleAmmoData _asfps_game_instance)))

(event EventWeaponFire
  (params (FireType :type FireType%20Enum :default "NewEnumerator0"))
  (bind _gunmesh (Variables|Default|GetGunMesh))
  (bind _returnvalue (Transformation|GetSocketTransform _gunmesh "AmmoEject" "RTS_World"))
  (|CallParentFunction FireType)
  (Components|Animation|PlayAnimation (Variables|Default|GetGunMesh) "/Game/MilitaryWeapSilver/Weapons/Animations/Fire_SniperRifle_W.Fire_SniperRifle_W" false)
  (if (Variables|Default|GetisAiming)
    (CallFunction|AutomaticRecoil)
    (else
      (Effects|SpawnEmitteratLocation "/Game/Particles/FX_SniperShell.FX_SniperShell" (.location _returnvalue) (.rotation _returnvalue)))))

(event EventWeaponReload
  (|CallParentFunction)
  (Audio|PlaySoundatLocation "/Game/MilitaryWeapSilver/Sound/SniperRifle/Wavs/SniperRifle_Reload03.SniperRifle_Reload03" (Transformation|GetWorldLocation (Variables|/Script/Engine.Character|GetMesh (Variables|Default|GetPlayerRef))) "0, 0, 0" 1.0 1.0 0.0 0 0 0))

(event EventOnAimEnter
  (bind _playerref (Variables|Default|GetPlayerRef))
  (bind _playerref_2 (Variables|Default|GetPlayerRef))
  (bind _sniperscoperef (Variables|/Game/Blueprints/FPS_Character.FPS_Character_C|GetSniperScopeRef _playerref))
  (|CallParentFunction)
  (if (== (Variables|/Game/Blueprints/FPS_Character.FPS_Character_C|GetCurrentWeapon (Variables|Default|GetPlayerRef)) self)
    (Variables|/Game/Blueprints/FPS_Character.FPS_Character_C|SetCanSwitchWeapon _playerref_2 false)
    (Variables|/Game/Blueprints/FPS_Character.FPS_Character_C|SetcanReload _playerref_2 false)
    (Utilities|FlowControl|Delay 0.1)
    (if (not (UserInterface|Viewport|IsinViewport _sniperscoperef))
      (UserInterface|Viewport|AddtoViewport _sniperscoperef 0)
      (Development|SetHiddeninGame (Variables|Default|GetGunMesh) true false)
      (Rendering|SetActorHiddenInGame (Game|Player|GetPlayerPawn 0) true)
      (Widget|SetVisibility (Variables|/Game/Blueprints/FPS_Character.FPS_Character_C|GetMainHudRef (Variables|Default|GetPlayerRef)) "Collapsed")
      (Variables|Default|SetBulletSpread 0.0)
      (Variables|Default|SetRecoilIntesity 3e+01))))

(event EventOnAimExit
  (bind _playerref (Variables|Default|GetPlayerRef))
  (|CallParentFunction)
  (Variables|/Game/Blueprints/FPS_Character.FPS_Character_C|SetCanSwitchWeapon _playerref true)
  (Variables|/Game/Blueprints/FPS_Character.FPS_Character_C|SetcanReload _playerref true)
  (Widget|RemovefromParent (Variables|/Game/Blueprints/FPS_Character.FPS_Character_C|GetSniperScopeRef _playerref))
  (Development|SetHiddeninGame (Variables|Default|GetGunMesh) false false)
  (Rendering|SetActorHiddenInGame (Game|Player|GetPlayerPawn 0) false)
  (Widget|SetVisibility (Variables|/Game/Blueprints/FPS_Character.FPS_Character_C|GetMainHudRef (Variables|Default|GetPlayerRef)) "Visible")
  (Variables|Default|SetBulletSpread 8e+02)
  (Variables|Default|SetRecoilIntesity 6e+01))

(fn ConstructionScript
  (|CallParentFunction))