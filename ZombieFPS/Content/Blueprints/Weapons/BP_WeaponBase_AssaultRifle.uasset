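; Assault rifle child weapon that adds fully automatic fire to its parent weapon class, loading its ammo data from the game instance on BeginPlay.
; Firing starts a looping timer that runs the parent shot, gun animation, shell ejection and player fire call until stopped, or until empty, which triggers a reload.
; Aiming removes bullet spread and lowers recoil, and reloading wraps the parent logic with rifle sounds.
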(event Custom|RifleFire
  (bind _gunmesh (Variables|Default|GetGunMesh))
  (bind _returnvalue (Transformation|GetSocketTransform _gunmesh "AmmoEject" "RTS_World"))
  (if (Variables|Default|GetisRifleFiring)
    (|CallParentFunction (stale EventWeaponFire FireType))
    (Components|Animation|PlayAnimation (Variables|Default|GetGunMesh) "/Game/MilitaryWeapSilver/Weapons/Animations/Fire_Rifle_W.Fire_Rifle_W" false)
    (Effects|SpawnEmitteratLocation "/Game/Particles/FX_AssaultShell.FX_AssaultShell" (.location _returnvalue) (.rotation _returnvalue))
    (Default|CallCharacterFireWeapon (Variables|Default|GetPlayerRef) "NewEnumerator1")
    (if (<= (Variables|Default|GetCurrentAmmo) 0)
      (CallFunction|StopFire)
      (Default|Reload (Variables|Default|GetPlayerRef)))))

(event EventBeginPlay
  (|CallParentFunction)
  (bind _asfps_game_instance (Utilities|Casting|CastToFPS_GameInstance (Game|GetGameInstance)))
  (Variables|Default|SetAmmoData (Variables|/Game/Blueprints/FPS_GameInstance.FPS_GameInstance_C|GetAssaultRifleAmmoData _asfps_game_instance)))

(event Collision|EventActorBeginOverlap
  (params (OtherActor :type Actor%20Object%20Reference))
  (|CallParentFunction OtherActor) ; This node is disabled and will not be called.\nDrag off pins to build functionality.
)

(event EventTick
  (params (DeltaSeconds :type Float%20%28single-precision%29))
  (|CallParentFunction DeltaSeconds) ; This node is disabled and will not be called.\nDrag off pins to build functionality.
)

(event EventStopFire
  (|CallParentFunction)
  (Variables|Default|SetisRifleFiring false)
  (Utilities|Time|ClearandInvalidateTimerbyHandle (Variables|Default|GetRifleFireTimerHandle)))

(event EventWeaponReload
  (Audio|PlaySoundatLocation "/Game/MilitaryWeapSilver/Sound/Rifle/Wavs/Rifle_Lower.Rifle_Lower" (Transformation|GetWorldLocation (Variables|/Script/Engine.Character|GetMesh (Variables|Default|GetPlayerRef))) "0, 0, 0" 1.0 1.0 0.0 0 0 0)
  (|CallParentFunction)
  (Audio|PlaySoundatLocation "/Game/MilitaryWeapSilver/Sound/Rifle/Wavs/Rifle_Reload03.Rifle_Reload03" (Transformation|GetWorldLocation (Variables|/Script/Engine.Character|GetMesh (Variables|Default|GetPlayerRef))) "0, 0, 0" 1.0 1.0 0.0 0 0 0))

(event EventOnAimEnter
  (Variables|Default|SetBulletSpread 0.0)
  (Variables|Default|SetRecoilIntesity 7.0)
  (|CallParentFunction))

(event EventOnAimExit
  (Variables|Default|SetBulletSpread 5e+02)
  (Variables|Default|SetRecoilIntesity 15.0)
  (|CallParentFunction))

(event EventWeaponFire
  (params (FireType :type FireType%20Enum :default "NewEnumerator0"))
  (Variables|Default|SetisRifleFiring true)
  (CallFunction|RifleFire)
  (bind _returnvalue (Utilities|Time|SetTimerbyEvent (delegate Custom|RifleFire) (Variables|Default|GetAutomaticFireRate) true))
  (Variables|Default|SetRifleFireTimerHandle _returnvalue))

(fn ConstructionScript
  (|CallParentFunction))